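; BP_ReSpawn is a checkpoint actor that sets the current player start tag when a ThirdPersonCharacter overlaps its sphere.
; On overlap it resets the mesh material on every BP_ReSpawn in the level, then gives its own mesh a different one, marking it active.
; It then writes its PlayerStartTag to CurrentPlayerStartTag on ThirdPersonGameMode and prints the tag.
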(event OnComponentBeginOverlap(Sphere)
  (params (OverlappedComponent :type Primitive%20Component%20Object%20Reference) (OtherActor :type Actor%20Object%20Reference) (OtherComp :type Primitive%20Component%20Object%20Reference) (OtherBodyIndex :type Integer) (bFromSweep :type Boolean) (SweepResult :type Hit%20Result%20Structure%20%28by%20ref%29))
  (bind _playerstarttag (Variables|Default|GetPlayerStartTag))
  (Utilities|Casting|CastToThirdPersonCharacter OtherActor)
  (CallFunction|SetAllReSpawnMaterial)
  (Rendering|Material|SetMaterial (Variables|Default|GetStaticMesh) 0 "/Game/StarterContent/Materials/M_Brick_Clay_New.M_Brick_Clay_New")
  (Variables|/Game/ThirdPersonBP/Blueprints/ThirdPersonGameMode.ThirdPersonGameMode_C|SetCurrentPlayerStartTag (.AsThird%20Person%20Game%20Mode (Utilities|Casting|CastToThirdPersonGameMode (Game|GetGameMode))) _playerstarttag)
  (Development|PrintString (Utilities|String|ToString(Name) _playerstarttag)))

(fn ConstructionScript)

(fn SetAllReSpawnMaterial
  (bind _outactors (Actor|GetAllActorsOfClass "BP_ReSpawn_C"))
  (for _array_element _outactors
    (Rendering|Material|SetMaterial (Variables|BP_ReSpawn_C|GetStaticMesh _array_element) 0 "/Game/StarterContent/Materials/M_Tech_Hex_Tile.M_Tech_Hex_Tile")))